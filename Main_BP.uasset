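; Player character Blueprint with double jump, dash attack, countdown timer and end-of-game handling.
; Tick uses a retriggered-safe Delay as a one-second clock, showing scoreboard and pause menu and writing the leaderboard score at time-up.
; While jumping, a downward trace kills and bounces off enemies or dies on MonsterFlower; while dashing, a forward trace kills enemies.
; Tick also shows game-over and pause widgets when health runs out.
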(event `InputAction|ESC` :consume false
  (params (Key :type "Key Structure")))

(event `InputAxisKey|Gamepad_RightX`
  (params (AxisValue :type "Float (single-precision)"))
  (`self.AddControllerYawInput` (* AxisValue 1.0)))

(event `InputAction|Jump`
  (params (Key :type "Key Structure"))
  (bind _jumpcounter (`self.JumpCounter`))
  (:`Pressed`
    (bind _output_get (set `self.JumpEnabled` (`self.JumpEnabled`)))
    (if _output_get
      (set `self.IsJumping` true)
      (if (< _jumpcounter (`self.JumpMaxCount`))
        (bind _output_get_2 (set `self.JumpCounter` (+ _jumpcounter 1)))
        (if (>= _output_get_2 2)
          (`self.Jump`)
          (set `self.DoubleJump` true)
          (`KismetSystemLibrary.Delay` 0.2)
          (set `self.DoubleJump` false)
          (else
            (`self.Jump`))))))
  (:`Released`
    (`self.StopJumping`)))

(event `InputAction|Dash`
  (params (Key :type "Key Structure"))
  (:`Pressed`
    (bind _output_get (set `self.DashEnabled` (`self.DashEnabled`)))
    (if _output_get
      (set `self.IsDashing` true)
      (`KismetSystemLibrary.Delay` 0.75)
      (set `self.IsDashing` false))))

(event `self.OnLanded`
  (params (Hit :type "HitResult Structure (by ref)"))
  (set `self.JumpCounter` 0)
  (set `self.DoubleJump` false)
  (set `self.IsJumping` false))

(event `self.ReceiveTick`
  (params (DeltaSeconds :type "Float (single-precision)"))
  (bind _returnvalue (`self.K2_GetActorLocation` self))
  (`|ExecutionSequence`
    (:`then_0`
      (`KismetSystemLibrary.Delay` 1.0)
      (if (== (`self.Seconds`) 0)
        (if (== (`self.Minutes`) 0)
          (bind _output_get (set `self.TimeUp` (`self.TimeUp`)))
          (if _output_get
            (`WidgetLayoutLibrary.RemoveAllWidgets`)
            (bind _returnvalue_2 (`|CreateWidget` "/Game/HUD/ScoreBoard.ScoreBoard_C"))
            (`UserWidget.AddToViewport` _returnvalue_2 0)
            (`GameplayStatics.SetGamePaused` true)
            (`KismetSystemLibrary.Delay` 0.1)
            (set `PlayerController.bShowMouseCursor` true (`GameplayStatics.GetPlayerController` 0))
            (`WidgetBlueprintLibrary.SetInputMode_GameAndUIEx` (`GameplayStatics.GetPlayerController` 0) _returnvalue_2)
            (`WidgetLayoutLibrary.RemoveAllWidgets`)
            (bind _returnvalue_3 (`|CreateWidget` "/Game/HUD/PauseMenu.PauseMenu_C" (`GameplayStatics.GetPlayerController` 0)))
            (`UserWidget.AddToViewport` _returnvalue_3 0)
            (`Widget.SetVisibility` _returnvalue_3 "Visible")
            (`WidgetBlueprintLibrary.SetInputMode_GameAndUIEx` (`GameplayStatics.GetPlayerController` 0) _returnvalue_3)
            (`KismetSystemLibrary.Delay` 0.2)
            (`Widget.SetKeyboardFocus` (`/Game/HUD/PauseMenu.RestartLevelButton` _returnvalue_3))
            (bind _returnvalue_4 (`/Game/HUD/ScoreBoard.CalculatePointTotal` (`self.Target`)))
            (`LeaderboardBlueprintLibrary.WriteLeaderboardInteger` (`self.MainController`) "Score" _returnvalue_4)
            (set `self.TimeUp` false))
          (else
            (set `self.Seconds` 59)
            (set `self.Minutes` (- (`self.Minutes`) 1))))
        (else
          (set `self.Seconds` (- (`self.Seconds`) 1)))))
    (:`then_1`
      (if (`self.IsJumping`)
        (bind _outhit (`KismetSystemLibrary.LineTraceSingleForObjects` _returnvalue (+ (* (`self.GetActorUpVector` self) -150.0) _returnvalue) (`|MakeArray` "ObjectTypeQuery3" :!type "EObjectTypeQuery Enum")))
        (bind (_bblockinghit _binitialoverlap _time _distance _location _impactpoint _normal _impactnormal _physmat _hitactor) (`GameplayStatics.BreakHitResult` _outhit))
        (`KismetSystemLibrary.PrintString` (`KismetSystemLibrary.GetDisplayName` _hitactor) true true (struct :`G` 0.66 :`B` 1.0 :`A` 1.0) 10.0)
        (`|ExecutionSequence`
          (:`then_0`
            (bind _asmonster_flower_a_bp (cast `/Game/Enemies/MonsterFlowers/MonsterFlower_A_BP` _hitactor))
            (if (== _hitactor _asmonster_flower_a_bp)
              (`self.Die`)))
          (:`then_1`
            (bind _asenemy (cast `Enemy` _hitactor))
            (`self.LaunchCharacter` (0.0 0.0 1000.0))
            (`self.PlayAnimMontage` "/Game/Character/BunnyCombatMontage.BunnyCombatMontage" 1.0 "None")
            (`GameplayStatics.PlaySoundAtLocation` "/Game/ActionMusicSfxPack1/WAVs/Sound_FX/Action_Sound_FX/FX/FX1_Blip.FX1_Blip" (`self.K2_GetActorLocation`) (struct) 1.0 1.0 0.0 null null null)
            (bind _returnvalue_5 (`GameplayStatics.SpawnEmitterAtLocation` "/Game/SoulCity/EffectsMobileOpt/Smoke/ParticleSystems/P_smokeColumn.P_smokeColumn" (`self.K2_GetActorLocation` _asenemy) (struct) (0.5 0.5 0.5)))
            (`self.K2_DestroyActor` _asenemy)
            (`KismetSystemLibrary.Delay` 1.5)
            (`ActorComponent.K2_DestroyComponent` _returnvalue_5)
            (`self.IncrementKills` (`self.Amount`))))
        (elif (`self.IsDashing`)
          (`self.Dash`)
          (bind _asenemy_2 (cast `Enemy` (`self.HitActor`)))
          (bind _returnvalue_6 (`GameplayStatics.SpawnEmitterAtLocation` "/Game/SoulCity/EffectsMobileOpt/Smoke/ParticleSystems/P_smokeColumn.P_smokeColumn" (`self.K2_GetActorLocation` _asenemy_2) (struct) (0.5 0.5 0.5)))
          (`GameplayStatics.PlaySoundAtLocation` "/Game/ActionMusicSfxPack1/WAVs/Sound_FX/Action_Sound_FX/FX/FX1_Blip.FX1_Blip" (`self.K2_GetActorLocation`) (struct) 1.0 1.0 0.0 null null null)
          (`self.K2_DestroyActor` _asenemy_2)
          (`KismetSystemLibrary.Delay` 1.5)
          (`ActorComponent.K2_DestroyComponent` _returnvalue_6)
          (`self.IncrementKills` (`self.Amount`)))))
    (:`then_2`
      (if (<= (`self.Health`) 0.0)
        (bind _output_get_2 (set `self.GameOver` (`self.GameOver`)))
        (if _output_get_2
          (bind _returnvalue_7 (`|CreateWidget` "/Game/HUD/GameOver.GameOver_C" (`GameplayStatics.GetPlayerController` 0)))
          (`UserWidget.AddToViewport` _returnvalue_7 0)
          (`KismetSystemLibrary.Delay` 2.0)
          (`WidgetLayoutLibrary.RemoveAllWidgets`)
          (set `self.GameOver` false)
          (bind _returnvalue_8 (`|CreateWidget` "/Game/HUD/PauseMenu.PauseMenu_C" (`GameplayStatics.GetPlayerController` 0)))
          (`UserWidget.AddToViewport` _returnvalue_8 0)
          (`WidgetBlueprintLibrary.SetInputMode_GameAndUIEx` (`GameplayStatics.GetPlayerController` 0) null)
          (`KismetSystemLibrary.Delay` 0.2)
          (`Widget.SetKeyboardFocus` (`/Game/HUD/PauseMenu.RestartLevelButton` _returnvalue_8)))))))

(fn `Dash`
  (bind _returnvalue (`self.K2_GetActorLocation` self))
  (set `self.IsDashing` true)
  (`self.LaunchCharacter` (* (`self.GetActorForwardVector`) 200.0))
  (`self.PlayAnimMontage` "/Game/Character/BunnyCombatMontage.BunnyCombatMontage" 1.0 "Dash")
  (bind _outhit (`KismetSystemLibrary.LineTraceSingleForObjects` _returnvalue (+ (* (`self.GetActorForwardVector` self) 300.0) _returnvalue) (`|MakeArray` "ObjectTypeQuery3" :!type "EObjectTypeQuery Enum")))
  (set `self.HitActor` (`.HitActor` (`GameplayStatics.BreakHitResult` _outhit))))

(fn `MainJump`
  (bind _jumpcounter (`self.JumpCounter`))
  (bind _returnvalue (`self.K2_GetActorLocation` self))
  (bind _returnvalue_2 (`self.K2_GetActorLocation` self))
  (if (< _jumpcounter (`self.JumpMaxCount`))
    (bind _output_get (set `self.JumpCounter` (+ _jumpcounter 1)))
    (if (>= _output_get 2)
      (`self.Jump`)
      (set `self.DoubleJump` true)
      (bind _outhit (`KismetSystemLibrary.LineTraceSingleForObjects` _returnvalue (+ (* (`self.GetActorUpVector` self) -600.0) _returnvalue) (`|MakeArray` "ObjectTypeQuery3" :!type "EObjectTypeQuery Enum")))
      (set `self.HitActor` (`.HitActor` (`GameplayStatics.BreakHitResult` _outhit)))
      (else
        (`self.Jump`)
        (bind _outhit_2 (`KismetSystemLibrary.LineTraceSingleForObjects` _returnvalue_2 (+ (* (`self.GetActorUpVector` self) -600.0) _returnvalue_2) (`|MakeArray` "ObjectTypeQuery3" :!type "EObjectTypeQuery Enum")))
        (set `self.HitActor` (`.HitActor` (`GameplayStatics.BreakHitResult` _outhit_2)))))))

(fn `UserConstructionScript`)